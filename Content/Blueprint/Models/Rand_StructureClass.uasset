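; Base mining structure whose slave workers extract resources from its biome into the player's inventory, configured by type from RandStructureDB at construction.
; Slave count changes refresh the allowed resources present in the biome and restart mining; Tick starts new cycles when RestTime runs out.
; Each cycle picks a random resource, animates during a timed delay, then yields one unit per slave, dropping the resource when GetResource returns true.
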(event `self.ReceiveBeginPlay`
  (`parent.ReceiveBeginPlay`))

(event `self.ReceiveTick`
  (params (DeltaSeconds :type "Float (single-precision)"))
  (`parent.ReceiveTick` 0.0)
  (if (and (and (> (`self.CurSlaveAmount`) 0) (<= (`self.RestTime`) 0.0)) (> (`KismetArrayLibrary.Array_Length` (`self.CurAllowedRes`)) 0))
    (`self.Search and Mine`)))

(event `self.SlaveAmount has been changed`
  (`self.CheckBiomeResources`)
  (`self.Search and Mine`))

(event `Search and Mine`
  (bind _delaytime (`self.CountDelayTime`))
  (`KismetSystemLibrary.K2_ClearAndInvalidateTimerHandle` (`self.TimerHandle`))
  (set `self.RestTime` _delaytime)
  (bind _canmine (`self.CanMine`))
  (if _canmine
    (`self.Start/StopAnim` true)
    (bind _returnvalue (`KismetSystemLibrary.K2_SetTimer` null "MineResource" _delaytime))
    (set `self.TimerHandle` _returnvalue)
    (else
      (`KismetSystemLibrary.K2_ClearAndInvalidateTimerHandle` (`self.TimerHandle`))
      (set `self.RestTime` 0.0))))

(fn `CanMine`
  (returns (CanMine :type Boolean))
  (bind _curallowedres (`self.CurAllowedRes`))
  (if (and (> (`self.CurSlaveAmount`) 0) (> (`KismetArrayLibrary.Array_Length` (`self.CurAllowedRes`)) 0))
    (set `self.CurRes` (cast `/Game/Blueprint/Structures/Resources/ResourceType` (`|GetArrayItem` _curallowedres (`KismetMathLibrary.RandomInteger` (`KismetArrayLibrary.Array_LastIndex` _curallowedres)))))
    (return true)
    (else
      (`KismetSystemLibrary.PrintString` "Can't mine" true true (struct :`R` 1.0 :`G` 0.898209 :`A` 1.0))
      (set `self.CurRes` "NewEnumerator0")
      (return false))))

(fn `CheckBiomeResources`
  (`KismetArrayLibrary.Array_Clear` (`self.CurAllowedRes`))
  (bind _result (`BlueprintSetLibrary.Set_ToArray` (`self.AllowedResources`)))
  (for _array_element _result
    (if (`.ReturnValue` (`BlueprintMapLibrary.Map_Find` (`/Game/Blueprint/Models/BiomeClass.Current Resources` (`self.BiomeClass`)) _array_element))
      (`KismetArrayLibrary.Array_Add` (`self.CurAllowedRes`) _array_element))))

(fn `MineResource`
  (bind _curres (`self.CurRes`))
  (for _ (range (`self.CurSlaveAmount`))
    (bind _thelast (`/Game/Blueprint/Models/BiomeClass.GetResource` (`self.BiomeClass`) _curres))
    (`/Game/Blueprint/Scripts/Player/BP_Player.AddResInventory` (`self.BpPlayer`) (make `/Game/Blueprint/Structures/Biomes/ResAmount` _curres 1))
    (if _thelast
      (`KismetArrayLibrary.Array_RemoveItem` (`self.CurAllowedRes`) _curres)
      (break)))
  (set `self.RestTime` 0.0)
  (`self.Start/StopAnim` false))

(fn `UserConstructionScript`
  (bind (_name _description _texture _baseresorces _explosivesamount _slaveamount _time _allowedbiomes _allowedresources _polutionpoints) (break `/Game/Blueprint/Structures/Stcuctures/RandStructureData` (`BlueprintMapLibrary.Map_Find` (`self.RandStructureDB`) (`self.RandType`))))
  (`parent.UserConstructionScript`)
  (set `self.Base Resources` _baseresorces)
  (set `self.ExplodesAmount` _explosivesamount)
  (set `self.MaxSlaveAmount` _slaveamount)
  (set `self.DelayTime` (`KismetMathLibrary.Conv_IntToDouble` _time))
  (set `self.AllowedBiomes` _allowedbiomes)
  (set `self.AllowedResources` _allowedresources)
  (set `self.StructTexture` _texture)
  (set `self.Name` _name)
  (set `self.Description` _description)
  (set `self. PollutionPoints` _polutionpoints))