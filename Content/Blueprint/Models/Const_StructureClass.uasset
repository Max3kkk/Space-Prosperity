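; Constructed structure class that turns the player's inventory resources into recipe outputs while slaves are assigned to it.
; The construction script loads its stats and recipes from ConstStructureDB by ConstType, flagging zero-time structures as one-off grants paid on BeginPlay once the game has started.
; Otherwise, Tick and slave-count changes check workers and inputs, then TryRecipe sets a timer from CountDelayTime for DoRecipe to exchange the resources.
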(event `self.ReceiveBeginPlay`
  (`parent.ReceiveBeginPlay`)
  (if (`/Game/Blueprint/Scripts/Player/BP_Player.GameStarted` (`self.BpPlayer`))
    (if (`self.IsOnceWorking`)
      (`/Game/Blueprint/Scripts/Player/BP_Player.AddResInventory` (`self.BpPlayer`) (`self.Once Giving Res`)))))

(event `self.ReceiveTick`
  (params (DeltaSeconds :type "Float (single-precision)"))
  (`parent.ReceiveTick` DeltaSeconds)
  (bind _out (`self.CheckSlaveAmount`))
  (if (and _out (<= (`self.RestTime`) 0.0))
    (bind _cando (`self.CheckRecipe` (`self.Recipe Index`)))
    (if _cando
      (`self.TryRecipe`))))

(event `self.SlaveAmount has been changed`
  (bind _out (`self.CheckSlaveAmount`))
  (if _out
    (bind _cando (`self.CheckRecipe` (`self.Recipe Index`)))
    (if _cando
      (`self.TryRecipe`))))

(event `TryRecipe`
  (bind _recipe_index (`self.Recipe Index`))
  (bind _delaytime (`self.CountDelayTime`))
  (set `self.RestTime` _delaytime)
  (bind _out (`self.CheckSlaveAmount`))
  (if _out
    (bind _cando (`self.CheckRecipe` _recipe_index))
    (if _cando
      (set `self.CurRes` (`.ResourceType_3_D77A5A43443F996587FB959BBED1CFD3` (break `/Game/Blueprint/Structures/Biomes/ResAmount` (`.OutcomingResource_17_7B7BE04A449DF7233A203483409F4919` (break `/Game/Blueprint/Structures/Stcuctures/Recipe` (`|GetArrayItem` (`self.Recipes`) _recipe_index))))))
      (bind _returnvalue (`KismetSystemLibrary.K2_SetTimer` null "DoRecipe" _delaytime))
      (set `self.TimerHandle` _returnvalue)
      (else
        (set `self.CurRes` "NewEnumerator0" :!label _label)
        (`KismetSystemLibrary.K2_ClearAndInvalidateTimerHandle` (`self.TimerHandle`))
        (set `self.RestTime` 0.0)))
    (else
      (goto _label))))

(fn `CheckRecipe`
  (params (Index :type Integer))
  (returns (CanDo :type Boolean))
  (set `self.IsThereAll` true)
  (for _array_element (`.IncomingResources_9_9136E0664C42F1F83AE976B1EFF8B2A4` (break `/Game/Blueprint/Structures/Stcuctures/Recipe` (`|GetArrayItem` (`self.Recipes`) Index)))
    (bind _isthere (`/Game/Blueprint/Scripts/Player/BP_Player.CheckResInventory` (`self.BpPlayer`) _array_element))
    (if (not _isthere)
      (set `self.IsThereAll` false)
      (break)))
  (return (`self.IsThereAll`)))

(fn `CheckSlaveAmount`
  (returns (Out :type Boolean))
  (return (and (not (`self.IsOnceWorking`)) (> (`self.CurSlaveAmount`) 0))))

(fn `DoRecipe`
  (bind (_incomingresources _outcomingresource) (break `/Game/Blueprint/Structures/Stcuctures/Recipe` (`|GetArrayItem` (`self.Recipes`) (`self.Recipe Index`))))
  (if (> (`KismetArrayLibrary.Array_Length` _incomingresources) 0)
    (for _array_element _incomingresources
      (`/Game/Blueprint/Scripts/Player/BP_Player.RemoveResInventory` (`self.BpPlayer`) _array_element)
      (`/Game/Blueprint/Scripts/Player/BP_Player.AddResInventory` (`self.BpPlayer`) _outcomingresource :!label _label)
      (set `self.RestTime` 0.0 :!label _label_2))
    (else
      (goto _label)))
  (goto _label_2))

(fn `UserConstructionScript`
  (bind (_texture _baseresorces _explosivesamount _slaveamount _time _allowedbiomes _recipes) (break `/Game/Blueprint/Structures/Stcuctures/ConstStructureData` (`BlueprintMapLibrary.Map_Find` (`self.ConstStructureDB`) (`self.ConstType`))))
  (`parent.UserConstructionScript`)
  (set `self.StructTexture` (`.Texture_29_E994A0114F757665118FE5A568A8A304` (break `/Game/Blueprint/Structures/Stcuctures/ConstStructureData` (`BlueprintMapLibrary.Map_Find` (`self.ConstStructureDB`) (`self.ConstType`)))))
  (set `self.Base Resources` _baseresorces)
  (set `self.ExplodesAmount` _explosivesamount)
  (set `self.MaxSlaveAmount` _slaveamount)
  (set `self.DelayTime` (`KismetMathLibrary.Conv_IntToDouble` _time))
  (set `self.AllowedBiomes` _allowedbiomes)
  (set `self.Recipes` _recipes)
  (if (== (`self.DelayTime`) 0.0)
    (set `self.Once Giving Res` (`.OutcomingResource_17_7B7BE04A449DF7233A203483409F4919` (break `/Game/Blueprint/Structures/Stcuctures/Recipe` (`|GetArrayItem` (`self.Recipes`)))))
    (set `self.IsOnceWorking` true)))