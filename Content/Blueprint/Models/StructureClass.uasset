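; StructureClass is a structure actor Blueprint that tracks how many workers are assigned to it and shows that count visually.
; AddWorker and RemoveWorker adjust the count and call RefreshWorkerModels.
; RefreshWorkerModels destroys the current worker actor and, when the count is nonzero, spawns the class mapped to that count in the WorkerModels map at the structure's transform.
; BeginPlay only casts the player pawn to BP_Player.
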(event `self.ReceiveBeginPlay`
  (cast `/Game/Blueprint/Scripts/Player/BP_Player` (`GameplayStatics.GetPlayerPawn` 0)))

(fn `AddWorker`
  (`/Engine/EditorBlueprintResources/StandardMacros.IncrementInt` (`self.CurWorkerAmount`)
    (:`  `
      (`self.RefreshWorkerModels`)
      (return))))

(fn `RefreshWorkerModels`
  (bind _curworkeramount (`self.CurWorkerAmount`))
  (if (`KismetSystemLibrary.IsValid` (`self.CurWorkerActor`))
    (`self.K2_DestroyActor` (`self.CurWorkerActor`)))
  (if (!= _curworkeramount 0)
    (bind _returnvalue (`|SpawnActorFromClass` (`BlueprintMapLibrary.Map_Find` (`self.WorkerModels`) _curworkeramount) (`self.GetTransform` self) "Undefined" "OverrideRootScale" null null))
    (set `self.CurWorkerActor` _returnvalue)))

(fn `RemoveWorker`
  (`/Engine/EditorBlueprintResources/StandardMacros.DecrementInt` (`self.CurWorkerAmount`)
    (:`  `
      (`self.RefreshWorkerModels`)
      (return))))

(fn `UserConstructionScript`)