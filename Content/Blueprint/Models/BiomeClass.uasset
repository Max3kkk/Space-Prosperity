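; Biome tile actor for a planet, holding randomly generated solid and liquid resources, a worker model and an optional structure.
; Initialization reads flat or volume biome tables for display, flattening and terraforming data, rolls resources and may spawn a random structure on unchanged flat tiles.
; Resource changes update the remaining percentage.
; Terraforming (costing player resources) and flattening replace the actor, copying neighbours and state; only terraforming carries over the resource percentage.
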(event `self.ReceiveBeginPlay`
  (if (not (`self.ChangedBiome`))
    _))

(event `Terraform Biome`
  (bind _newbiome (`self.NewBiome`))
  (bind (_canterraform _resource _finalbiome _isflat) (break `/Game/Blueprint/Structures/Biomes/Terraforming` (`self.Terraforming Data`)))
  (bind _asbp_player (cast `/Game/Blueprint/Scripts/Player/BP_Player` (`GameplayStatics.GetPlayerCharacter` 0)))
  (`/Game/Blueprint/Scripts/Player/BP_Player.RemoveResInventory` _asbp_player _resource)
  (`self.SpawnOtherBiome` _asbp_player _isflat _finalbiome
    (:`Out`
      (`self.Share Biome Data` _newbiome
        (:`Out`
          (`/Game/Blueprint/Scripts/Player/BP_Player.RefreshSelectedBiome` _asbp_player _newbiome)
          (`self.K2_DestroyActor`))))))

(fn `AddResource`
  (params (ResAmount :type "/Game/Blueprint/Structures/Biomes/ResAmount Structure"))
  (bind (_resourcetype _amount) (break `/Game/Blueprint/Structures/Biomes/ResAmount` ResAmount))
  (bind _current_resources (`self.Current Resources`))
  (bind (_value _returnvalue) (`BlueprintMapLibrary.Map_Find` _current_resources _resourcetype))
  (bind _returnvalue_2 (`KismetMathLibrary.FFloor` (* (/ (`KismetMathLibrary.Conv_IntToDouble` (+ (`self.Solid Res`) (`self.Liquid Res`))) (`KismetMathLibrary.Conv_IntToDouble` (`self.MaxResAmount`))) 100.0)))
  (if _returnvalue
    (`BlueprintMapLibrary.Map_Add` (`self.Current Resources`) _resourcetype (+ _value _amount))
    (`self.RefreshResAmount` _resourcetype)
    (set `self.Percent of res` _returnvalue_2)
    (else
      (`BlueprintMapLibrary.Map_Add` _current_resources _resourcetype _amount)
      (`self.RefreshResAmount` _resourcetype)
      (set `self.Percent of res` _returnvalue_2))))

(fn `Flat`
  (bind _newbiome (`self.NewBiome`))
  (bind (_canflat _mintime _maxtime _finalbiome _isflat) (break `/Game/Blueprint/Structures/Biomes/Flatting` (`self.Flatting Data`)))
  (bind _asbp_player (cast `/Game/Blueprint/Scripts/Player/BP_Player` (`GameplayStatics.GetPlayerCharacter` 0)))
  (`self.SpawnOtherBiome` _asbp_player _isflat _finalbiome
    (:`Out`
      (`self.Share Biome Data` _newbiome false
        (:`Out`
          (`/Game/Blueprint/Scripts/Player/BP_Player.RefreshSelectedBiome` _asbp_player _newbiome)
          (`self.K2_DestroyActor`))))))

(fn `Generate Resources`
  (set `self.Liquid Res` 0)
  (set `self.Solid Res` 0)
  (`BlueprintMapLibrary.Map_Clear` (`self.Current Resources`))
  (for _index (range (+ (`KismetArrayLibrary.Array_LastIndex` (`self.Resources Data`)) 1))
    (bind (_resourcetype _minamount _maxamount _percent) (break `/Game/Blueprint/Structures/Biomes/ResPercenrt` (`|GetArrayItem` (`self.Resources Data`) _index)))
    (if (>= _percent (`KismetMathLibrary.RandomIntegerInRange` 1 100))
      (bind _returnvalue (/ (* (`KismetMathLibrary.RandomIntegerInRange` _minamount _maxamount) (`self.Percent of res`)) 100))
      (`BlueprintMapLibrary.Map_Add` (`self.Current Resources`) _resourcetype _returnvalue)
      (bind _returnvalue_2 (`self.Is Liquid` _resourcetype))
      (if _returnvalue_2
        (bind _output_get (set `self.Liquid Res` (+ (`self.Liquid Res`) _returnvalue)))
        (else
          (bind _output_get_2 (set `self.Solid Res` (+ (`self.Solid Res`) _returnvalue)))))
      (set `self.MaxResAmount` (+ _output_get_2 _output_get)))))

(fn `GetResource`
  (params (ResType :type "/Game/Blueprint/Structures/Resources/ResourceType Enum" :default "NewEnumerator0"))
  (returns (TheLast :type Boolean))
  (bind _current_resources (`self.Current Resources`))
  (bind _value (`BlueprintMapLibrary.Map_Find` _current_resources ResType))
  (bind _returnvalue (`KismetMathLibrary.FFloor` (* (/ (`KismetMathLibrary.Conv_IntToDouble` (+ (`self.Solid Res`) (`self.Liquid Res`))) (`KismetMathLibrary.Conv_IntToDouble` (`self.MaxResAmount`))) 100.0)))
  (if (<= _value 1)
    (`BlueprintMapLibrary.Map_Remove` (`self.Current Resources`) ResType)
    (`self.RefreshResAmount` ResType)
    (set `self.Percent of res` _returnvalue)
    (return true)
    (else
      (`BlueprintMapLibrary.Map_Add` _current_resources ResType (- _value 1))
      (`self.RefreshResAmount` ResType)
      (set `self.Percent of res` _returnvalue)
      (return false))))

(fn `Initialization`
  (if (`self.IsFlat`)
    (bind (_flatting _terraforming) (`self.SetData` (`self.FlatBiomeDB`)))
    (`self.SetTerraformingData` _terraforming)
    (`self.SetFlattingData` _flatting)
    (`self.SetData+` (`self.FlatBiomedb+`))
    (`self.PlaceRandomHealthStruct`)
    (else
      (bind (_flatting_2 _terraforming_2) (`self.SetData` (`self.BiomeDB`)))
      (`self.SetTerraformingData` _terraforming_2)
      (`self.SetFlattingData` _flatting_2)
      (`self.SetData+` (`self.BiomeDB+`))))
  (`self.Generate Resources`))

(fn `Is Liquid`
  (params (Resource :type "/Game/Blueprint/Structures/Resources/ResourceType Enum" :default "NewEnumerator0"))
  (returns (ReturnValue :type Boolean))
  (return (or (or (or (`|EnumEquality` Resource "NewEnumerator14") (`|EnumEquality` Resource "NewEnumerator15")) (`|EnumEquality` Resource "NewEnumerator16")) (`|EnumEquality` Resource "NewEnumerator33"))))

(fn `PlaceRandomHealthStruct`
  (locals (Percent :type Integer :default 0))
  (if (and (not (`self.ChangedBiome`)) (and (`self.IsFlat`) (not (`self.HasStructure`))))
    (set `local.Percent` (`KismetMathLibrary.RandomIntegerInRange` 1 100))
    (for _array_element (`.Percents_13_C6D438284AB66F061885549085E582DD` (break `/Game/Blueprint/Structures/Stcuctures/Perc+StructArray` (`BlueprintMapLibrary.Map_Find` (`self.FlatBiomeHealthStrDB`) (`self.BiomeType`))))
      (bind (_min _max _structure) (break `/Game/Blueprint/Structures/Stcuctures/Perc+Struct` _array_element))
      (if (`KismetMathLibrary.InRange_IntInt` (`local.Percent`) _min _max false)
        (bind _returnvalue (`|SpawnActorFromClass` _structure (`self.GetTransform` self) "AlwaysSpawn" "OverrideRootScale" null null))
        (bind _output_get (set `/Game/Blueprint/Models/StructureClass.BiomeClass` self _returnvalue))
        (set `/Game/Blueprint/Models/BiomeClass.HasStructure` true _output_get)
        (set `self.Structure` _returnvalue)
        (break)))))

(fn `RefreshResAmount`
  (params (Resource :type "/Game/Blueprint/Structures/Resources/ResourceType Enum" :default "NewEnumerator0"))
  (bind _returnvalue (`self.Is Liquid` Resource))
  (if _returnvalue
    (bind _result (`/Engine/EditorBlueprintResources/StandardMacros.DecrementInt` (`self.Liquid Res`))
      (:`  `
        _))
    (else
      (bind _result_2 (`/Engine/EditorBlueprintResources/StandardMacros.DecrementInt` (`self.Solid Res`))
        (:`  `
          _))))
  (set `self.Percent of res` (`KismetMathLibrary.Round` (* (/ (`KismetMathLibrary.Conv_IntToDouble` (+ _result _result_2)) (`KismetMathLibrary.Conv_IntToDouble` (`self.MaxResAmount`))) 100.0))))

(fn `RefreshWorkers`
  (bind _curslaveamount (`self.CurSlaveAmount`))
  (if (`KismetSystemLibrary.IsValid` (`self.CurSlaveActor`))
    (`self.K2_DestroyActor` (`self.CurSlaveActor`)))
  (if (!= _curslaveamount 0)
    (bind _returnvalue (`|SpawnActorFromClass` (`BlueprintMapLibrary.Map_Find` (`self.SlaveModels`) _curslaveamount) (`self.GetTransform` self) "Undefined" "OverrideRootScale" null null))
    (set `self.CurSlaveActor` _returnvalue)))

(fn `SetData`
  (params (BD :type "Map of /Game/Blueprint/Structures/Biomes/BiomeType Enum to /Game/Blueprint/Structures/Biomes/BiomeData Structure (by ref)" :default _))
  (returns (Flatting :type "/Game/Blueprint/Structures/Biomes/Flatting Structure") (Terraforming :type "/Game/Blueprint/Structures/Biomes/Terraforming Structure"))
  (bind (_resources _flatting _terraforming) (break `/Game/Blueprint/Structures/Biomes/BiomeData` (`BlueprintMapLibrary.Map_Find` BD (`self.BiomeType`))))
  (bind (_canflat _mintime _maxtime _finalbiome _isflat) (break `/Game/Blueprint/Structures/Biomes/Flatting` _flatting))
  (set `self.Resources Data` _resources)
  (bind _output_get (set `self.Flatting Data` (make `/Game/Blueprint/Structures/Biomes/Flatting` _canflat 0 (`KismetMathLibrary.RandomIntegerInRange` _mintime _maxtime) _finalbiome _isflat)))
  (bind _output_get_2 (set `self.Terraforming Data` _terraforming))
  (return _output_get _output_get_2))

(fn `SetData+`
  (params (`BD+` :type "Map of /Game/Blueprint/Structures/Biomes/BiomeType Enum to /Game/Blueprint/Structures/Biomes/BiomeData+ Structure (by ref)" :default _))
  (bind (_name _texture _description) (break `/Game/Blueprint/Structures/Biomes/BiomeData+` (`BlueprintMapLibrary.Map_Find` `BD+` (`self.BiomeType`))))
  (set `self.Name` _name)
  (set `self.Texture` _texture)
  (set `self.Description` _description))

(fn `SetFlattingData`
  (params (Flatting :type "/Game/Blueprint/Structures/Biomes/Flatting Structure (by ref)"))
  (bind (_canflat _mintime _maxtime _finalbiome _isflat) (break `/Game/Blueprint/Structures/Biomes/Flatting` Flatting))
  (bind (_name _texture _description) (break `/Game/Blueprint/Structures/Biomes/BiomeData+` (`BlueprintMapLibrary.Map_Find` (`self.BiomeDB+`) _finalbiome)))
  (bind (_name_2 _texture_2 _description_2) (break `/Game/Blueprint/Structures/Biomes/BiomeData+` (`BlueprintMapLibrary.Map_Find` (`self.FlatBiomedb+`) _finalbiome)))
  (if _canflat
    (if _isflat
      (set `self.Flatting Data+` (make `/Game/Blueprint/Structures/Biomes/BiomeData+` _name_2 _texture_2 _description_2))
      (else
        (set `self.Flatting Data+` (make `/Game/Blueprint/Structures/Biomes/BiomeData+` _name _texture _description))))))

(fn `SetTerraformingData`
  (params (Terraforming :type "/Game/Blueprint/Structures/Biomes/Terraforming Structure (by ref)"))
  (bind (_canterraform _resource _finalbiome _isflat) (break `/Game/Blueprint/Structures/Biomes/Terraforming` Terraforming))
  (bind (_name _texture _description) (break `/Game/Blueprint/Structures/Biomes/BiomeData+` (`BlueprintMapLibrary.Map_Find` (`self.BiomeDB+`) _finalbiome)))
  (bind (_name_2 _texture_2 _description_2) (break `/Game/Blueprint/Structures/Biomes/BiomeData+` (`BlueprintMapLibrary.Map_Find` (`self.FlatBiomedb+`) _finalbiome)))
  (if _canterraform
    (if _isflat
      (set `self.TerraformingData+` (make `/Game/Blueprint/Structures/Biomes/BiomeData+` _name_2 _texture_2 _description_2))
      (else
        (set `self.TerraformingData+` (make `/Game/Blueprint/Structures/Biomes/BiomeData+` _name _texture _description))))))

(fn `UserConstructionScript`
  (`self.SetActorHiddenInGame` false)
  (`self.SetActorEnableCollision` true))