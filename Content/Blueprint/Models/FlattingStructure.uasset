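; Flattening structure on a biome: assigned slaves mine its resources into the player's inventory until the structure flattens the biome and explodes.
; A named timer, paused while no slaves are assigned, triggers flattening, as does finding the biome empty when picking a random resource.
; Each mining cycle waits out a calculated delay with animation, grants up to one unit per slave, then Tick starts the next.
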(event `StartTimer`
  (bind _returnvalue (`KismetSystemLibrary.K2_SetTimer` self "Flatting" (`self.MaxTime`)))
  (set `self.TimerHandle` _returnvalue)
  (`self.MineResource`))

(event `self.SlaveAmount has been changed`
  (`self.MineResource`))

(event `self.ReceiveTick`
  (params (DeltaSeconds :type "Float (single-precision)"))
  (if (<= (`self.RestTime`) 0.0)
    (`self.MineResource`)))

(event `MineResource`
  (bind _curres (`self.CurRes`))
  (if (> (`self.CurSlaveAmount`) 0)
    (if (`|EnumEquality` _curres "NewEnumerator0")
      (`self.RandRes` :!label _label
        (:`Out`
          _))
      (else
        (bind _can (`self.CanMineRes` _curres))
        (if _can
          _
          (else
            (goto _label)))))
    (`KismetSystemLibrary.K2_UnPauseTimerHandle` (`self.TimerHandle`))
    (bind _delaytime (`self.CountDelayTime`))
    (bind _output_get (set `self.RestTime` _delaytime))
    (`self.Start/StopAnim` true)
    (`KismetSystemLibrary.RetriggerableDelay` _output_get)
    (`self.MineRes`)
    (else
      (`KismetSystemLibrary.K2_PauseTimerHandle` (`self.TimerHandle`))
      (`self.Start/StopAnim` false))))

(fn `CanMineRes`
  (params (Resource :type "/Game/Blueprint/Structures/Resources/ResourceType Enum" :default "NewEnumerator0"))
  (returns (Can :type Boolean))
  (bind (_value _returnvalue) (`BlueprintMapLibrary.Map_Find` (`/Game/Blueprint/Models/BiomeClass.Current Resources` (`self.BiomeClass`)) Resource))
  (return (and (> _value 0) _returnvalue)))

(fn `Flatting`
  (`/Game/Blueprint/Models/BiomeClass.Flat` (`self.BiomeClass`))
  (`self.Explode`))

(fn `Init`
  (params (Time :type "Float (double-precision)") (Biome :type "/Game/Blueprint/Models/BiomeClass Object Reference"))
  (set `self.MaxTime` Time)
  (set `self.BiomeClass` Biome)
  (bind _asbp_player (cast `/Game/Blueprint/Scripts/Player/BP_Player` (`GameplayStatics.GetPlayerCharacter` 0)))
  (set `self.BpPlayer` _asbp_player)
  (`self.StartTimer`))

(fn `TimerRemainingTime`
  (returns (RemainingTime :type "Float (double-precision)") (MaxTime :type "Float (double-precision)"))
  (return (`KismetSystemLibrary.K2_GetTimerRemainingTimeHandle` (`self.TimerHandle`)) (`self.MaxTime`)))

(fn `UserConstructionScript`
  (set `self.DelayTime` 10.0)
  (set `self.MaxSlaveAmount` 3))