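; Resource structure with finite health that produces randomized resources while slaves work it, then explodes when depleted.
; The construction script loads its stats from HealthStructDB by type, randomizing max health.
; Tick and slave-count changes trigger timed cycles that roll a weighted resource, pay the player amounts scaled by slave count, and drain health proportionally.
; A chance-based bonus resource goes to the biome or player, either at BeginPlay or on destruction.
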(event `self.ReceiveBeginPlay`
  (`parent.ReceiveBeginPlay`)
  (`self.ProduceFirstRes`))

(event `self.ReceiveTick`
  (params (DeltaSeconds :type "Float (single-precision)"))
  (`parent.ReceiveTick` DeltaSeconds)
  (bind _out (`self.CheckSlaveAmout`))
  (if (and _out (<= (`self.RestTime`) 0.0))
    (`self.TryRes`)))

(event `self.SlaveAmount has been changed`
  (bind _out (`self.CheckSlaveAmout`))
  (if _out
    (`self.TryRes`)))

(event `TryRes`
  (bind _delaytime (`self.CountDelayTime`))
  (bind _out (`self.CheckSlaveAmout`))
  (if _out
    (`self.Start/StopAnim` true)
    (`self.RandRes`
      (:`Out`
        (bind _output_get (set `self.RestTime` _delaytime))
        (bind _returnvalue (`KismetSystemLibrary.K2_SetTimer` null "ProduceRes" _output_get))
        (set `self.TimerHandle` _returnvalue)))
    (else
      (set `self.CurRes` "NewEnumerator0")
      (`KismetSystemLibrary.K2_ClearAndInvalidateTimerHandle` (`self.TimerHandle`)))))

(fn `CheckSlaveAmout`
  (returns (Out :type Boolean))
  (return (> (`self.CurSlaveAmount`) 0)))

(fn `ExplodeHealthStructure`
  (set `self.CurHealth` 0)
  (`self.ProduceLastRes`)
  (`self.Explode`))

(fn `ProduceFirstRes`
  (bind (_startafterdeath _biomeinventory _resource) (break `/Game/Blueprint/Structures/Stcuctures/LastRes` (`self.LastRes`)))
  (bind (_resourcetype _minamount _maxamount _percent) (break `/Game/Blueprint/Structures/Biomes/ResPercenrt` _resource))
  (bind _returnvalue (`KismetMathLibrary.RandomIntegerInRange` _minamount _maxamount))
  (if (and (<= (`KismetMathLibrary.RandomInteger` 100) _percent) (not _startafterdeath))
    (if (not _biomeinventory)
      (`/Game/Blueprint/Models/BiomeClass.AddResource` (`self.BiomeClass`) (make `/Game/Blueprint/Structures/Biomes/ResAmount` _resourcetype _returnvalue))
      (else
        (`/Game/Blueprint/Scripts/Player/BP_Player.AddResInventory` (`self.BpPlayer`) (make `/Game/Blueprint/Structures/Biomes/ResAmount` _resourcetype _returnvalue))))))

(fn `ProduceLastRes`
  (bind (_startafterdeath _biomeinventory _resource) (break `/Game/Blueprint/Structures/Stcuctures/LastRes` (`self.LastRes`)))
  (bind (_resourcetype _minamount _maxamount _percent) (break `/Game/Blueprint/Structures/Biomes/ResPercenrt` _resource))
  (bind _returnvalue (`KismetMathLibrary.RandomIntegerInRange` _minamount _maxamount))
  (if (and (<= (`KismetMathLibrary.RandomInteger` 100) _percent) _startafterdeath)
    (if (not _biomeinventory)
      (`/Game/Blueprint/Models/BiomeClass.AddResource` (`self.BiomeClass`) (make `/Game/Blueprint/Structures/Biomes/ResAmount` _resourcetype _returnvalue))
      (else
        (`/Game/Blueprint/Scripts/Player/BP_Player.AddResInventory` (`self.BpPlayer`) (make `/Game/Blueprint/Structures/Biomes/ResAmount` _resourcetype _returnvalue))))))

(fn `ProduceRes`
  (locals (Percent :type Integer) (ResAmount :type "/Game/Blueprint/Structures/Biomes/ResAmount Structure"))
  (bind (_resourcetype _amount) (break `/Game/Blueprint/Structures/Biomes/ResAmount` (`self.Resource`)))
  (`/Game/Blueprint/Scripts/Player/BP_Player.AddResInventory` (`self.BpPlayer`) (make `/Game/Blueprint/Structures/Biomes/ResAmount` _resourcetype (* _amount (`self.CurSlaveAmount`))))
  (`self.ReduceHealth`)
  (set `self.RestTime` 0.0)
  (`self.Start/StopAnim` false))

(fn `ReduceHealth`
  (bind _returnvalue (- (`self.CurHealth`) (* (`self.CurSlaveAmount`) 5)))
  (if (<= _returnvalue 0)
    (`self.ExplodeHealthStructure`)
    (else
      (set `self.CurHealth` _returnvalue))))

(fn `UserConstructionScript`
  (bind (_name _description _texture _minhealth _maxhealth _explosivesamount _maxslaveamount _delaytime _resources _lastres _allowedbiomes _baseresources _hasanimation) (break `/Game/Blueprint/Structures/Stcuctures/HealthStructureData` (`BlueprintMapLibrary.Map_Find` (`self.HealthStructDB`) (`self.HealthStructType`))))
  (`parent.UserConstructionScript`)
  (set `self.StructTexture` _texture)
  (bind _output_get (set `self.MaxHealth` (`KismetMathLibrary.RandomIntegerInRange` _minhealth _maxhealth)))
  (set `self.CurHealth` _output_get)
  (set `self.ExplodesAmount` _explosivesamount)
  (set `self.MaxSlaveAmount` _maxslaveamount)
  (set `self.DelayTime` (`KismetMathLibrary.Conv_IntToDouble` _delaytime))
  (set `self.Resources` _resources)
  (set `self.LastRes` _lastres)
  (set `self.AllowedBiomes` _allowedbiomes)
  (set `self.Base Resources` _baseresources)
  (set `self.Name` _name)
  (set `self.Description` _description)
  (set `self.HasAnimation` _hasanimation))