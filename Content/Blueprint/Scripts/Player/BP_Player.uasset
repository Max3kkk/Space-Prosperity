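; Player pawn for a planet colony builder, with RMB-gated orbit camera, wheel zoom, click biome selection and panel toggles.
; Game start reveals a random biome and its neighbours by moving them into place and destroying closed placeholders, then grants base resources.
; An enum-keyed inventory map tracks resources and caps assigned slave workers.
; Helpers spawn structures on the selected biome, start timed flattening, and terraform by swapping in flat ground actors.
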(event `Key|MouseScrollUp`
  (params (Key :type "Key Structure"))
  (bind _camera_boom (`self.Camera Boom`))
  (bind _targetarmlength (`SpringArmComponent.TargetArmLength` _camera_boom))
  ;[1 1 1] Приближение/Удаление
  (:`Pressed`
    (if (>= _targetarmlength 7000.0)
      (set `SpringArmComponent.TargetArmLength` (- _targetarmlength 250.0) _camera_boom))))

(event `InputAction|PressRMB`
  (params (Key :type "Key Structure"))
  ;[1 1 1] Вверх/Вниз Влево/Вправо
  (:`Pressed`
    (goto _label :!via `Open`))
  (:`Released`
    (goto _label :!via `Close`)))

(event `InputAxis|MoveHorizontal`
  (params (AxisValue :type "Float (single-precision)"))
  ;[1 1 1] Вверх/Вниз Влево/Вправо
  (`/Engine/EditorBlueprintResources/StandardMacros.Gate` true :!label _label
    (:`Exit`
      (`self.AddControllerYawInput` AxisValue))))

(event `Key|MouseScrollDown`
  (params (Key :type "Key Structure"))
  (bind _camera_boom (`self.Camera Boom`))
  (bind _targetarmlength (`SpringArmComponent.TargetArmLength` _camera_boom))
  ;[1 1 1] Приближение/Удаление
  (:`Pressed`
    (if (<= _targetarmlength 20000.0)
      (set `SpringArmComponent.TargetArmLength` (+ _targetarmlength 250.0) _camera_boom))))

(event `InputAction|PressRMB`
  (params (Key :type "Key Structure"))
  ;[1 1 1] Вверх/Вниз Влево/Вправо
  (:`Pressed`
    (goto _label_2 :!via `Open`))
  (:`Released`
    (goto _label_2 :!via `Close`)))

(event `InputAxis|MoveVertical`
  (params (AxisValue :type "Float (single-precision)"))
  ;[1 1 1] Вверх/Вниз Влево/Вправо
  (`/Engine/EditorBlueprintResources/StandardMacros.Gate` true :!label _label_2
    (:`Exit`
      (`self.AddControllerPitchInput` AxisValue))))

(event `InputAction|OpenStructurePanel`
  (params (Key :type "Key Structure"))
  ;[1 1 1] Open/Hide StructurePanel
  (:`Pressed`
    (`/Game/UI/Custom/StructurePanel/StructurePanel.Open/Close Panel` (`self.StructurePanel`) false true)))

(event `InputAction|OpenBiomePanel`
  (params (Key :type "Key Structure"))
  ;[1 1 1] Open/Hide BiomePanel
  (:`Pressed`
    (`/Game/UI/Custom/Biome_Str_Panel/Biome/BiomeInfoPanel.Hide/OpenPanel` (`self.BiomeInfoPanel`))))

(event `InputAction|PressLMB`
  (params (Key :type "Key Structure"))
  (bind (_hitresult _returnvalue) (`PlayerController.GetHitResultUnderCursorForObjects` (`GameplayStatics.GetPlayerController` 0) (`|MakeArray` "ObjectTypeQuery2" :!type "EObjectTypeQuery Enum") true))
  (bind (_bblockinghit _binitialoverlap _time _distance _location _impactpoint _normal _impactnormal _physmat _hitactor) (`GameplayStatics.BreakHitResult` _hitresult))
  ;[1 1 1] Biome Openning
  (:`Pressed`
    (`/Engine/EditorBlueprintResources/StandardMacros.Gate` true :!label _label_3
      (:`Exit`
        (if _returnvalue
          (bind _as_2733_closed (cast `/Game/Blueprint/Models/Biomes/_2733_Closed` _hitactor)
            (:`CastFailed`
              (bind _as_3090_closed (cast `/Game/Blueprint/Models/Biomes/_3090_Closed` _hitactor)
                (:`CastFailed`
                  (bind _asbiome_class (cast `/Game/Blueprint/Models/BiomeClass` _hitactor))
                  (`self.Neighbour openning` _asbiome_class))))))))))

(event `InputAction|PressLMB`
  (params (Key :type "Key Structure"))
  (bind (_hitresult _returnvalue) (`PlayerController.GetHitResultUnderCursorForObjects` (`GameplayStatics.GetPlayerController` 0) (`|MakeArray` "ObjectTypeQuery2" :!type "EObjectTypeQuery Enum") true))
  (bind (_bblockinghit _binitialoverlap _time _distance _location _impactpoint _normal _impactnormal _physmat _hitactor) (`GameplayStatics.BreakHitResult` _hitresult))
  ;[1 1 1] SelectBiome
  (:`Pressed`
    (if _returnvalue
      (cast `/Game/Blueprint/Models/Biomes/_2733_Closed` _hitactor
        (:`CastFailed`
          (cast `/Game/Blueprint/Models/Biomes/_3090_Closed` _hitactor
            (:`CastFailed`
              (bind _asbiome_class (cast `/Game/Blueprint/Models/BiomeClass` _hitactor))
              (`self.RefreshSelectedBiome` _asbiome_class))))))))

(event `InputAction|OpenSomeLocs`
  (params (Key :type "Key Structure"))
  ;[1 1 1] Biome Openning
  (:`Pressed`
    (goto _label_3 :!via `Open`))
  (:`Released`
    (goto _label_3 :!via `Close`)))

(event `InputAction|SelectBiome`
  (params (Key :type "Key Structure"))
  ;[1 1 1] SelectBiome
  (:`Pressed`
    (`/Engine/EditorBlueprintResources/StandardMacros.Gate` true :!via `Open` :!label _label_4))
  (:`Released`
    (goto _label_4 :!via `Close`)))

(fn `AddResInventory`
  (params (ResAmount :type "/Game/Blueprint/Structures/Biomes/ResAmount Structure"))
  (bind (_resourcetype _amount) (break `/Game/Blueprint/Structures/Biomes/ResAmount` ResAmount))
  (bind _inventory (`self.Inventory`))
  (bind (_name _texture _description _amount_2 _isopened) (break `/Game/Blueprint/Structures/Resources/ResourceData` (`BlueprintMapLibrary.Map_Find` _inventory _resourcetype)))
  (`BlueprintMapLibrary.Map_Add` _inventory _resourcetype (make `/Game/Blueprint/Structures/Resources/ResourceData` _name _texture _description (+ _amount _amount_2) _isopened))
  (`self.OpenRes` _resourcetype))

(fn `BaseResourceAdding`
  (bind _enumvalue (foreach `/Game/Blueprint/Structures/Resources/ResourceType` false)
    (:`LoopBody`
      (bind (_value _returnvalue) (`BlueprintMapLibrary.Map_Find` (`self.Base Resources`) _enumvalue))
      (if _returnvalue
        (`self.AddResInventory` (make `/Game/Blueprint/Structures/Biomes/ResAmount` _enumvalue _value)))
      (`self.GameStarted Event`)
      (set `self.GameStarted` true))))

(fn `BeginPlay`
  (`self.Random Biome Openning`)
  (`self.BaseResourceAdding`))

(fn `BuildStructure`
  (params (Rand :type "/Game/Blueprint/Structures/Stcuctures/RandStrucType Enum" :default "NewEnumerator9") (Const :type "/Game/Blueprint/Structures/Stcuctures/ConstStrucType Enum" :default "NewEnumerator9") (Health :type "/Game/Blueprint/Structures/Stcuctures/HealthStructType Enum" :default "NewEnumerator3"))
  (bind _selectedbiome (`self.SelectedBiome`))
  (bind _selectedbiome_2 (`self.SelectedBiome`))
  (bind _selectedbiome_3 (`self.SelectedBiome`))
  (if (`|EnumInequality` Rand "NewEnumerator9")
    (bind _returnvalue (`|SpawnActorFromClass` (`BlueprintMapLibrary.Map_Find` (`self.RandStructureBd`) Rand) (`/Game/Blueprint/Models/BiomeClass.BiomTransform` (`self.SelectedBiome`)) "Undefined" "OverrideRootScale" null null))
    (bind _output_get (set `/Game/Blueprint/Models/BiomeClass.Structure` _returnvalue _selectedbiome_3))
    (set `/Game/Blueprint/Models/BiomeClass.HasStructure` true _selectedbiome_3)
    (set `/Game/Blueprint/Models/StructureClass.BiomeClass` _selectedbiome_3 _output_get)
    (`/Game/Blueprint/Models/Rand_StructureClass.CheckBiomeResources` _returnvalue)
    (`self.Neighbour openning` (`self.SelectedBiome`) :!label _label)
    (elif (`|EnumInequality` Const "NewEnumerator9")
      (bind _returnvalue_2 (`|SpawnActorFromClass` (`BlueprintMapLibrary.Map_Find` (`self.ConstStructureBd`) Const) (`/Game/Blueprint/Models/BiomeClass.BiomTransform` (`self.SelectedBiome`)) "Undefined" "OverrideRootScale" null null))
      (bind _output_get_2 (set `/Game/Blueprint/Models/BiomeClass.Structure` _returnvalue_2 _selectedbiome_2))
      (set `/Game/Blueprint/Models/BiomeClass.HasStructure` true _selectedbiome_2)
      (set `/Game/Blueprint/Models/StructureClass.BiomeClass` _selectedbiome_2 _output_get_2)
      (goto _label)
      (elif (`|EnumInequality` Health "NewEnumerator3")
        (bind _returnvalue_3 (`|SpawnActorFromClass` (`BlueprintMapLibrary.Map_Find` (`self.HealthStructureBd`) Health) (`/Game/Blueprint/Models/BiomeClass.BiomTransform` (`self.SelectedBiome`)) "Undefined" "OverrideRootScale" null null))
        (bind _output_get_3 (set `/Game/Blueprint/Models/BiomeClass.Structure` _returnvalue_3 _selectedbiome))
        (set `/Game/Blueprint/Models/BiomeClass.HasStructure` true _selectedbiome)
        (set `/Game/Blueprint/Models/StructureClass.BiomeClass` _selectedbiome _output_get_3)))))

(fn `CheckResInventory`
  (params (ResAmount :type "/Game/Blueprint/Structures/Biomes/ResAmount Structure"))
  (returns (IsThere :type Boolean))
  (bind (_resourcetype _amount) (break `/Game/Blueprint/Structures/Biomes/ResAmount` ResAmount))
  (bind (_value _returnvalue) (`BlueprintMapLibrary.Map_Find` (`self.Inventory`) _resourcetype))
  (if _returnvalue
    (if (>= (`.Amount_9_847A9D124583A86ECBAF53A2D0922F61` (break `/Game/Blueprint/Structures/Resources/ResourceData` _value)) _amount)
      (return true)
      (else
        (return false)))
    (else
      (return false))))

(fn `FreeWorker`
  (returns (IsThere :type Boolean))
  (if true
    (return (< (`self.WorkingSlaves`) (`.Amount_9_847A9D124583A86ECBAF53A2D0922F61` (break `/Game/Blueprint/Structures/Resources/ResourceData` (`BlueprintMapLibrary.Map_Find` (`self.Inventory`) "NewEnumerator34")))))
    (else
      (return false))))

(fn `Neighbour openning`
  (params (Biome :type "/Game/Blueprint/Models/BiomeClass Object Reference"))
  (bind _localneighbours (`self.LocalNeighbours`))
  (bind _checknone (`self.CheckNone`))
  (bind _closedparent (`/Game/Blueprint/Models/BiomeClass.ClosedParent` (`self.Biome`)))
  (bind _output_get (set `self.Biome` Biome))
  (set `self.LocalNeighbours` (`/Game/Blueprint/Models/BiomeClass.Neighbours` _output_get))
  (for _index (range (+ (`KismetArrayLibrary.Array_LastIndex` _localneighbours) 1))
    (bind _output (`|GetArrayItem` _localneighbours _index))
    (if (!= _output -1)
      (bind _output_get_2 (set `self.Biome` (`|GetArrayItem` (`/Game/Blueprint/Scripts/Planets/BasePlanet.Bioms` (`self.Planet`)) _output)))
      (bind _location (.location (`/Game/Blueprint/Models/BiomeClass.BiomTransform` _output_get_2)))
      (bind _rotation (.rotation (`/Game/Blueprint/Models/BiomeClass.BiomTransform` _output_get_2)))
      (`self.K2_SetActorTransform` _output_get_2 (`KismetMathLibrary.MakeTransform` _location _rotation) false false)
      (if (`/Game/Blueprint/Models/BiomeClass.HasStructure` _output_get_2)
        (`self.K2_SetActorTransform` (`/Game/Blueprint/Models/BiomeClass.Structure` _output_get_2) (`KismetMathLibrary.MakeTransform` _location _rotation) false false))
      (if (!= _closedparent _checknone)
        (`self.K2_DestroyActor` _closedparent)
        (set `/Game/Blueprint/Models/BiomeClass.ClosedParent` _checknone (`self.Biome`))))))

(fn `OneBiomeOpenning`
  (params (Biome :type "/Game/Blueprint/Models/BiomeClass Object Reference"))
  (bind _output_get (set `self.Biome` Biome))
  (bind _location (.location (`/Game/Blueprint/Models/BiomeClass.BiomTransform` _output_get)))
  (bind _rotation (.rotation (`/Game/Blueprint/Models/BiomeClass.BiomTransform` _output_get)))
  (`self.K2_SetActorTransform` _output_get (`KismetMathLibrary.MakeTransform` _location _rotation) false false)
  (if (`/Game/Blueprint/Models/BiomeClass.HasStructure` _output_get)
    (`self.K2_SetActorTransform` (`/Game/Blueprint/Models/BiomeClass.Structure` _output_get) (`KismetMathLibrary.MakeTransform` _location _rotation) false false))
  (set `self.LocalNeighbours` (`/Game/Blueprint/Models/BiomeClass.Neighbours` _output_get))
  (bind _output_get_2 (set `self.Biome` _output_get))
  (`self.K2_DestroyActor` (`/Game/Blueprint/Models/BiomeClass.ClosedParent` _output_get_2)))

(fn `PlaceCamera`
  (`self.K2_SetActorRotation` (.rotation (`self.StartTransform`))))

(fn `Random Biome Openning`
  (bind _biome (`self.Biome`))
  (bind _bioms (`/Game/Blueprint/Scripts/Planets/BasePlanet.Bioms` (`self.Planet`)))
  (bind _output_get (set `self.Biome` (`|GetArrayItem` _bioms (`KismetMathLibrary.RandomIntegerInRange` 0 (`KismetArrayLibrary.Array_LastIndex` _bioms)))))
  (set `self.StartTransform` (`/Game/Blueprint/Models/BiomeClass.BiomTransform` _output_get))
  (`self.OneBiomeOpenning` _output_get)
  (set `self.SelectedBiome` _biome)
  (`/Game/UI/Custom/Biome_Str_Panel/Biome/BiomeInfoPanel.RefreshPanel` (`self.BiomeInfoPanel`))
  (`self.Neighbour openning` _biome)
  (`self.PlaceCamera`))

(fn `RefreshSelectedBiome`
  (params (SelectedBiome :type "/Game/Blueprint/Models/BiomeClass Object Reference"))
  (bind _output_get (set `self.SelectedBiome` SelectedBiome))
  (`/Game/UI/Custom/Biome_Str_Panel/Biome/BiomeInfoPanel.RefreshPanel` (`self.BiomeInfoPanel`))
  (set `/Game/UI/Custom/StructurePanel/StructurePanel.SelectedBiome` _output_get (`self.StructurePanel`)))

(fn `RemoveExtraSlaves`
  (locals (ExtraAmount :type Integer :default 0) (`Cur Slave` :type Integer :default 0))
  (bind _workingslaves (`self.WorkingSlaves`))
  (bind _extraamount (`local.ExtraAmount`))
  (bind (_name _texture _description _amount) (break `/Game/Blueprint/Structures/Resources/ResourceData` (`BlueprintMapLibrary.Map_Find` (`self.Inventory`) "NewEnumerator34")))
  (if (> _workingslaves _amount)
    (set `local.ExtraAmount` (- _workingslaves _amount))
    (for _array_element (`self.StructureswithSlaves`)
      (bind _curslaveamount (`/Game/Blueprint/Models/StructureClass.CurSlaveAmount` _array_element))
      (bind _output_get (set `local.Cur Slave` _curslaveamount))
      (if (> _extraamount _curslaveamount)
        (`/Game/Blueprint/Models/StructureClass.Add/RemoveSlave` _array_element true _output_get false)
        (bind _output_get_2 (set `local.ExtraAmount` (- _extraamount (`local.Cur Slave`))))
        (if (<= _output_get_2 0)
          (break))
        (else
          (`/Game/Blueprint/Models/StructureClass.Add/RemoveSlave` _array_element true _extraamount false)
          (break))))
    (set `self.WorkingSlaves` _amount)))

(fn `RemoveResInventory`
  (params (ResAmount :type "/Game/Blueprint/Structures/Biomes/ResAmount Structure"))
  (bind (_resourcetype _amount) (break `/Game/Blueprint/Structures/Biomes/ResAmount` ResAmount))
  (bind _inventory (`self.Inventory`))
  (bind (_name _texture _description _amount_2 _isopened) (break `/Game/Blueprint/Structures/Resources/ResourceData` (`BlueprintMapLibrary.Map_Find` _inventory _resourcetype)))
  (`BlueprintMapLibrary.Map_Add` _inventory _resourcetype (make `/Game/Blueprint/Structures/Resources/ResourceData` _name _texture _description (- _amount_2 _amount) _isopened))
  (`self.OpenRes` _resourcetype))

(fn `StartBiomeFlatting`
  (params (Biome :type "/Game/Blueprint/Models/BiomeClass Object Reference"))
  (bind _returnvalue (`|SpawnActorFromClass` (`self.FlattingStructure`) (`/Game/Blueprint/Models/BiomeClass.BiomTransform` Biome) "Undefined" "OverrideRootScale" null null))
  (bind _asflatting_structure (cast `/Game/Blueprint/Models/Structures/Others/FlattingStructure` _returnvalue))
  (`/Game/Blueprint/Models/Structures/Others/FlattingStructure.Init` _asflatting_structure (`KismetMathLibrary.Conv_IntToDouble` (`.MaxTime_21_8E160E8D4994AF6D4B9A0EAA47E5B29D` (break `/Game/Blueprint/Structures/Biomes/Flatting` (`/Game/Blueprint/Models/BiomeClass.Flatting Data` Biome)))) Biome)
  (set `/Game/Blueprint/Models/BiomeClass.Structure` _asflatting_structure Biome)
  (set `/Game/Blueprint/Models/BiomeClass.HasStructure` false Biome)
  (set `/Game/Blueprint/Models/BiomeClass.IsChanging` true Biome))

(fn `UserConstructionScript`
  (if (== (`BlueprintMapLibrary.Map_Length` (`self.Inventory`)) 0)
    (bind _enumvalue (foreach `/Game/Blueprint/Structures/Resources/ResourceType` false)
      (:`LoopBody`
        (`BlueprintMapLibrary.Map_Add` (`self.Inventory`) _enumvalue (make `/Game/Blueprint/Structures/Resources/ResourceData` (`|GetEnumeratorNameAsString` _enumvalue)))))))