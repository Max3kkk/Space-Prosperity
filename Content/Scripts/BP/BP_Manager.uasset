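; Quest manager that steps through an ordered quest list, announcing descriptions and completion with on-screen prints.
; CheckQuest matches an actor to the current quest and caches it; СompleteQuest handles single or multi-actor objectives before advancing.
; PressE validates the cached actor's overlap and, for Talking or Interaction quests, distance, then calls CompleteQuest on that BP_QuestItem.
; Dialogue on/off calls are forwarded to BP_Player.
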(event `self.ReceiveBeginPlay`
  (`self.Initialize`))

(fn `CheckQuest`
  (params (Actor :type "Actor Object Reference"))
  (returns (Bool :type Boolean) (QuestType :type "/Game/Scripts/BP/QuestSystem/QuestType Enum"))
  (locals (Trigger :type "Actor Object Reference") (isUsed :type "Array of Boolean") (completedAmount :type Integer) (i :type Integer) (actorList :type "Array of Actor Object Reference") (isCompleted :type Boolean) (curQuestType :type "/Game/Scripts/BP/QuestSystem/QuestType Enum"))
  (bind _returnvalue (`KismetArrayLibrary.Array_Length` (`local.actorList`)))
  (set `local.Trigger` Actor)
  (bind _output_get (set `self.LastQuest` (`|GetArrayItem` (`self.QuestList`) (`self.QuestIndex`))))
  (bind (_description _type _actor _iscompleted _isused _completedamount) (break `/Game/Scripts/BP/QuestSystem/Quest` _output_get))
  (set `local.isUsed` _isused)
  (set `local.completedAmount` _completedamount)
  (set `local.actorList` _actor)
  (set `local.isCompleted` _iscompleted)
  (set `local.curQuestType` _type)
  (if (and (> _returnvalue 1) (> _returnvalue (`local.completedAmount`)))
    (for _index (range (`KismetArrayLibrary.Array_Length` (`local.actorList`)))
      (bind _output_get_2 (set `local.i` _index))
      (if (and (== (`|GetArrayItem` (`local.actorList`) (`local.i`)) (`local.Trigger`)) (not (`|GetArrayItem` (`local.isUsed`) _output_get_2)))
        (`KismetSystemLibrary.PrintString` "There is quest for this Actor" true true (struct :`G` 1.0 :`B` 0.184858 :`A` 1.0) 10.0)
        (set `self.LastActor` (`local.Trigger`))
        (return true (`local.curQuestType`))))
    (`KismetSystemLibrary.PrintString` "No quest for this Actor" true true (struct :`G` 0.434835 :`B` 1.0 :`A` 1.0) 10.0)
    (return false "NewEnumerator5")
    (elif (== (`|GetArrayItem` (`local.actorList`)) (`local.Trigger`))
      (`KismetSystemLibrary.PrintString` "There is quest for this Actor" true true (struct :`G` 1.0 :`B` 0.184858 :`A` 1.0))
      (set `self.LastActor` (`local.Trigger`))
      (return true (`local.curQuestType`))
      (else
        (`KismetSystemLibrary.PrintString` "No quest for this Actor" true true (struct :`G` 0.434835 :`B` 1.0 :`A` 1.0) 10.0)
        (return false "NewEnumerator5")))))

(fn `DialogueOff`
  (`/Game/Scripts/BP/Player/BP_Player.DialogueOff` (`self.BP Player`)))

(fn `DialogueOn`
  (params (Dialogue :type "/Game/Scripts/BP/QuestSystem/Dialogue Structure") (Actor :type "Actor Object Reference") (NPCName :type String))
  (`/Game/Scripts/BP/Player/BP_Player.DialogueOn` (`self.BP Player`) Dialogue Actor NPCName))

(fn `IsDistanceEnough`
  (params (Object :type "Object Object Reference") (Selection :type "/Game/Scripts/BP/QuestSystem/QuestType Enum" :default "NewEnumerator5") (Distance :type "Float (double-precision)"))
  (returns (`AsBP Quest Item` :type "/Game/Scripts/BP/QuestSystem/QuestPrefabs/BP_QuestItem Object Reference") (Bool :type Boolean))
  (bind _asbp_quest_item (cast `/Game/Scripts/BP/QuestSystem/QuestPrefabs/BP_QuestItem` Object))
  (switch `/Game/Scripts/BP/QuestSystem/QuestType` Selection
    (:`NewEnumerator0`
      _)
    (:`NewEnumerator1`
      (bind _returnvalue (>= (`/Game/Scripts/BP/QuestSystem/QuestPrefabs/BP_QuestItem.talkDistance` _asbp_quest_item) Distance))
      (if _returnvalue
        _
        (else
          _))
      (return _asbp_quest_item _returnvalue))
    (:`NewEnumerator2`
      (bind _returnvalue_2 (>= (`/Game/Scripts/BP/QuestSystem/QuestPrefabs/BP_QuestItem.interactDistance` _asbp_quest_item) Distance))
      (if _returnvalue_2
        _
        (else
          _))
      (return _asbp_quest_item _returnvalue_2))
    (:`NewEnumerator3`
      _))
  (return _asbp_quest_item true))

(fn `PressE`
  (params (Actor :type "Actor Object Reference") (Distance :type "Float (double-precision)"))
  (bind _lastactor (`self.LastActor`))
  (bind _lastactor_2 (`self.LastActor`))
  (`/Engine/EditorBlueprintResources/StandardMacros.IsValid` _lastactor
    (:`Is Valid`
      (bind (_bool _questtype) (`self.CheckQuest` _lastactor_2))
      (if (and (and (`self.IsOverlappingActor` _lastactor_2 (`self.Player`)) _bool) (== Actor _lastactor))
        (bind (_asbp_quest_item _bool_2) (`self.IsDistanceEnough` _lastactor _questtype Distance))
        (if _bool_2
          (`/Game/Scripts/BP/QuestSystem/QuestPrefabs/BP_QuestItem.CompleteQuest` _asbp_quest_item _questtype true))))))

(fn `QuestComplited`
  (`KismetSystemLibrary.PrintString` "QuestCompleted!!!" true true (struct :`R` 0.091597 :`G` 0.94027 :`B` 1.0 :`A` 1.0) 3.0)
  (bind _output_get (set `self.QuestIndex` (+ (`self.QuestIndex`) 1)))
  (if (>= _output_get (`KismetArrayLibrary.Array_Length` (`self.QuestList`)))
    (`KismetSystemLibrary.PrintString` "All Quest Completed!!!" true true (struct :`R` 1.0 :`G` 1.0 :`B` 1.0 :`A` 1.0) 15.0)
    (else
      (bind _output_get_2 (set `self.LastQuest` (`|GetArrayItem` (`self.QuestList`) (`self.QuestIndex`))))
      (`KismetSystemLibrary.PrintString` (`KismetTextLibrary.Conv_TextToString` (`.Description_4_E9C74EEB4E0148BC42675AB8C1A2A74C` (break `/Game/Scripts/BP/QuestSystem/Quest` _output_get_2))) true true (struct :`R` 1.0 :`G` 1.0 :`B` 1.0 :`A` 1.0) 10.0))))

(fn `UserConstructionScript`)

(fn `СompleteQuest`
  (params (Actor :type "Actor Object Reference"))
  (locals (Trigger :type "Actor Object Reference") (i :type Integer) (completedAmount :type Integer) (isUsed :type "Array of Boolean") (actorList :type "Array of Actor Object Reference") (isCompleted :type Boolean))
  (bind _returnvalue (`KismetArrayLibrary.Array_Length` (`local.actorList`)))
  (set `local.Trigger` Actor)
  (bind _output_get (set `self.LastQuest` (`|GetArrayItem` (`self.QuestList`) (`self.QuestIndex`))))
  (bind (_description _type _actor _iscompleted _isused _completedamount) (break `/Game/Scripts/BP/QuestSystem/Quest` _output_get))
  (set `local.isUsed` _isused)
  (set `local.completedAmount` _completedamount)
  (set `local.actorList` _actor)
  (set `local.isCompleted` _iscompleted)
  (if (and (> _returnvalue 1) (> _returnvalue (`local.completedAmount`)))
    (for _index (range (`KismetArrayLibrary.Array_Length` (`local.actorList`)))
      (bind _output_get_2 (set `local.i` _index))
      (if (and (== (`|GetArrayItem` (`local.actorList`) (`local.i`)) (`local.Trigger`)) (not (`|GetArrayItem` (`local.isUsed`) _output_get_2)))
        (`KismetArrayLibrary.Array_Set` (`local.isUsed`) (`local.i`))
        (`/Engine/EditorBlueprintResources/StandardMacros.IncrementInt` (`local.completedAmount`)
          (:`  `
            (break)))))
    (if (== (`local.completedAmount`) (`KismetArrayLibrary.Array_Length` (`local.actorList`)))
      (`self.QuestComplited`))
    (elif (== (`|GetArrayItem` (`local.actorList`)) (`local.Trigger`))
      (`self.QuestComplited`)
      (else
        (`KismetSystemLibrary.PrintString` "Wrong Actor Tried to Complete the Quest" true true (struct :`R` 1.0 :`A` 1.0) 10.0)))))