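; First-person player Blueprint handling movement, look, E-key interaction, NPC dialogue and the pause menu.
; E line-traces from the camera and passes the hit to BP_Manager, which also completes quests when dialogue ends.
; During dialogue, look input applies only if a predictive trace still hits the speaker within range.
; Pausing sets global time dilation and the look multiplier to zero.
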(event `self.ReceiveBeginPlay`
  (`self.CreatePauseMenu`)
  (`self.Initialize Variables`)
  (`self.CreateDialogueWidget`)
  (bind _asbp_game_instance (cast `/Game/Scripts/BP/BP_GameInstance` (`GameplayStatics.GetGameInstance`)))
  (set `self.SQ` (`/Game/Scripts/BP/BP_GameInstance.Shadow` _asbp_game_instance)))

(event `Key|E`
  (params (Key :type "Key Structure"))
  (bind _camera (`self.Camera`))
  (bind _returnvalue (`SceneComponent.K2_GetComponentLocation` _camera))
  ;[1 1 1] PRESS E ; Line Trace
  (:`Pressed`
    (bind _outhit (`KismetSystemLibrary.LineTraceSingle` :`Start` _returnvalue :`End` (+ _returnvalue (* (`SceneComponent.GetForwardVector` _camera) 10000.0)) :`TraceChannel` "TraceTypeQuery2" :`bTraceComplex` true :`DrawDebugType` "ForDuration"))
    (bind (_bblockinghit _binitialoverlap _time _distance _location _impactpoint _normal _impactnormal _physmat _hitactor) (`GameplayStatics.BreakHitResult` _outhit))
    (`/Game/Scripts/BP/BP_Manager.PressE` (`self.BP_Manager`) _hitactor _distance)))

(event `InputAxis|MoveForward`
  (params (AxisValue :type "Float (single-precision)"))
  ;[1 1 1 1 20] WASD Inputs
  (`self.AddMovementInput` (`self.GetActorForwardVector`) AxisValue))

(event `InputAxis|MoveRight`
  (params (AxisValue :type "Float (single-precision)"))
  ;[1 1 1 1 20] WASD Inputs
  (`self.AddMovementInput` (`self.GetActorRightVector`) AxisValue))

(event `InputAction|Test`
  (params (Key :type "Key Structure"))
  (:`Pressed`
    (`KismetSystemLibrary.PrintString` "Hello")))

(event `InputAxis|MoveHorizontal`
  (params (AxisValue :type "Float (single-precision)"))
  (bind _curdialogueactor (`self.curDialogueActor`))
  (bind _returnvalue (`SceneComponent.K2_GetComponentLocation` (`self.Camera`)))
  (if (`Widget.IsVisible` (`self.DialogueWidget`))
    (bind _outhit (`KismetSystemLibrary.LineTraceSingle` :`Start` _returnvalue :`End` (+ _returnvalue (* (`KismetMathLibrary.Conv_RotatorToVector` (`KismetMathLibrary.MakeRotator` (.roll (`SceneComponent.K2_GetComponentRotation` (`self.Camera`))) (.pitch (`SceneComponent.K2_GetComponentRotation` (`self.Camera`))) (+ AxisValue (.yaw (`SceneComponent.K2_GetComponentRotation` (`self.Camera`)))))) 10000.0)) :`TraceChannel` "TraceTypeQuery2" :`bTraceComplex` true :`DrawDebugType` "ForDuration" :`TraceColor` (struct :`R` 1.0 :`B` 0.878595 :`A` 1.0) :`TraceHitColor` (struct :`R` 0.087826 :`G` 0.317708 :`B` 0.088808 :`A` 1.0)))
    (bind (_bblockinghit _binitialoverlap _time _distance _location _impactpoint _normal _impactnormal _physmat _hitactor) (`GameplayStatics.BreakHitResult` _outhit))
    (if (== _hitactor _curdialogueactor)
      (bind (_asbp_quest_item _bool) (`/Game/Scripts/BP/BP_Manager.IsDistanceEnough` (`self.BP_Manager`) _curdialogueactor "NewEnumerator1" _distance))
      (if _bool
        (`self.AddControllerYawInput` AxisValue)))
    (else
      (`self.AddControllerYawInput` (* (`self.delta`) AxisValue)))))

(event `InputAxis|MoveVertical`
  (params (AxisValue :type "Float (single-precision)"))
  (bind _curdialogueactor (`self.curDialogueActor`))
  (bind _returnvalue (`SceneComponent.K2_GetComponentLocation` (`self.Camera`)))
  (if (`Widget.IsVisible` (`self.DialogueWidget`))
    (bind _outhit (`KismetSystemLibrary.LineTraceSingle` :`Start` _returnvalue :`End` (+ _returnvalue (* (`KismetMathLibrary.Conv_RotatorToVector` (`KismetMathLibrary.MakeRotator` (.roll (`SceneComponent.K2_GetComponentRotation` (`self.Camera`))) (+ AxisValue (.pitch (`SceneComponent.K2_GetComponentRotation` (`self.Camera`)))) (.yaw (`SceneComponent.K2_GetComponentRotation` (`self.Camera`))))) 1000.0)) :`TraceChannel` "TraceTypeQuery2" :`bTraceComplex` true :`DrawDebugType` "ForDuration" :`TraceColor` (struct :`R` 1.0 :`B` 0.878595 :`A` 1.0) :`TraceHitColor` (struct :`R` 0.087826 :`G` 0.317708 :`B` 0.088808 :`A` 1.0)))
    (bind (_bblockinghit _binitialoverlap _time _distance _location _impactpoint _normal _impactnormal _physmat _hitactor) (`GameplayStatics.BreakHitResult` _outhit))
    (if (== _hitactor _curdialogueactor)
      (bind (_asbp_quest_item _bool) (`/Game/Scripts/BP/BP_Manager.IsDistanceEnough` (`self.BP_Manager`) _curdialogueactor "NewEnumerator1" _distance))
      (if _bool
        (`self.AddControllerPitchInput` AxisValue)))
    (else
      (`self.AddControllerPitchInput` (* (`self.delta`) AxisValue)))))

(event `InputAction|PressMenu`
  (params (Key :type "Key Structure"))
  ;[1 1 1] Press and Pause Game
  (:`Pressed`
    (if (`self.Menu_Visible`)
      (`Widget.SetVisibility` (`self.Menu_Pause`) "Hidden")
      (set `self.Menu_Visible` false)
      (`GameplayStatics.SetGlobalTimeDilation` 1.0)
      (set `self.delta` 1.0)
      (else
        (`Widget.SetVisibility` (`self.Menu_Pause`) "Visible")
        (set `self.Menu_Visible` true)
        (`GameplayStatics.SetGlobalTimeDilation` 0.0)
        (set `self.delta` 0.0)))))

(event `InputAction|PressNextReplica`
  (params (Key :type "Key Structure"))
  (bind (_replicas _index) (break `/Game/Scripts/BP/QuestSystem/Dialogue` (`self.curDialogue`)))
  (bind (_replicas_2 _index_2) (break `/Game/Scripts/BP/QuestSystem/Dialogue` (`self.curDialogue`)))
  ;[1 1 1] Press Next Replcica
  (:`Pressed`
    (if (< _index_2 (`KismetArrayLibrary.Array_Length` _replicas_2))
      (bind _result (`/Engine/EditorBlueprintResources/StandardMacros.IncrementInt` _index)
        (:`  `
          (bind _output_get (set `self.curDialogue` (make `/Game/Scripts/BP/QuestSystem/Dialogue` _replicas _result)))
          (bind (_replicas_3 _index_3) (break `/Game/Scripts/BP/QuestSystem/Dialogue` _output_get))
          (if (< _index_3 (`KismetArrayLibrary.Array_Length` _replicas_3))
            (bind (_player _text) (break `/Game/Scripts/BP/QuestSystem/Replica` (`|GetArrayItem` _replicas_3 _index_3)))
            (`/Game/UI/UMG_Dialogue.NextReplica` (`self.DialogueWidget`) _player _text (`self.curNPCName`))
            (`KismetSystemLibrary.Delay` 0.5)
            (else
              (`self.DialogueOff`)
              (`/Game/Scripts/BP/BP_Manager.СompleteQuest` (`self.BP_Manager`) (`self.curDialogueActor`)))))))))

(fn `DialogueOff`
  (`Widget.SetVisibility` (`self.DialogueWidget`) "Hidden"))

(fn `DialogueOn`
  (params (Dialogue :type "/Game/Scripts/BP/QuestSystem/Dialogue Structure") (Actor :type "Actor Object Reference") (NPCName :type String))
  (bind _output_get (set `self.curDialogue` Dialogue))
  (set `self.curDialogueActor` Actor)
  (set `self.curNPCName` NPCName)
  (bind (_replicas _index) (break `/Game/Scripts/BP/QuestSystem/Dialogue` _output_get))
  (bind (_player _text) (break `/Game/Scripts/BP/QuestSystem/Replica` (`|GetArrayItem` _replicas _index)))
  (`/Game/UI/UMG_Dialogue.NextReplica` (`self.DialogueWidget`) _player _text (`self.curNPCName`))
  (`Widget.SetVisibility` (`self.DialogueWidget`) "Visible"))

(fn `UserConstructionScript`)