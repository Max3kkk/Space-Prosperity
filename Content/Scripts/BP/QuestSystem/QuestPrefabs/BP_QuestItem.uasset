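; Quest item actor that serves as a trigger, talk target or interactable for quests tracked by BP_Manager.
; When the player overlaps its box, it asks the manager for the quest type, completing Movement quests immediately or showing a text prompt for Talking and Interaction.
; With PressE set, CompleteQuest either sends the current DialogueList entry to the manager's dialogue or reports the interaction as complete.
; Ending overlap hides the prompt.
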(event `self.ReceiveBeginPlay`
  (`self.Reset`)
  (set `self.talkDistance` 120.0)
  (set `self.interactDistance` 400.0))

(event `self.BoxCollider.OnComponentBeginOverlap`
  (params (OverlappedComponent :type "PrimitiveComponent Object Reference") (OtherActor :type "Actor Object Reference") (OtherComp :type "PrimitiveComponent Object Reference") (OtherBodyIndex :type Integer) (bFromSweep :type Boolean) (SweepResult :type "HitResult Structure (by ref)"))
  (bind _asbp_player (cast `/Game/Scripts/BP/Player/BP_Player` OtherActor))
  (set `self.playerName` (`/Game/Scripts/BP/Player/BP_Player.Name` _asbp_player))
  (bind (_bool _questtype) (`/Game/Scripts/BP/BP_Manager.CheckQuest` (`self.BP_Manager`) self))
  (if _bool
    (`self.CompleteQuest` _questtype)))

(event `self.ReceiveActorEndOverlap`
  (params (OtherActor :type "Actor Object Reference"))
  (cast `/Game/Scripts/BP/Player/BP_Player` OtherActor)
  (`self.Reset`))

(fn `CompleteQuest`
  (params (QuestType :type "/Game/Scripts/BP/QuestSystem/QuestType Enum" :default "NewEnumerator5") (PressE :type Boolean :default false))
  (`self.Check to E Quest` QuestType)
  (if PressE
    (switch `/Game/Scripts/BP/QuestSystem/QuestType` QuestType
      (:`NewEnumerator1`
        (`self.Talk`))
      (:`NewEnumerator2`
        (`self.Interact`)))
    (else
      (switch `/Game/Scripts/BP/QuestSystem/QuestType` QuestType
        (:`NewEnumerator0`
          (`/Game/Scripts/BP/BP_Manager.СompleteQuest` (`self.BP_Manager`) self))))))

(fn `Interact`
  (`SceneComponent.SetVisibility` (`self.TextRender`) false false)
  (`/Game/Scripts/BP/BP_Manager.СompleteQuest` (`self.BP_Manager`) self))

(fn `Reset`
  (`SceneComponent.SetVisibility` (`self.TextRender`) false false)
  (`/Engine/EditorBlueprintResources/StandardMacros.IsValid` (`self.BP_Manager`)
    (:`Is Not Valid`
      (bind _asbp_manager (castclass `/Game/Scripts/BP/BP_Manager` "/Game/Scripts/BP/BP_Manager.BP_Manager_C"))
      (bind _outactors (`GameplayStatics.GetAllActorsOfClass` _asbp_manager))
      (set `self.BP_Manager` (`|GetArrayItem` _outactors)))))

(fn `Talk`
  (locals (LastDialogue :type "/Game/Scripts/BP/QuestSystem/Dialogue Structure"))
  (`SceneComponent.SetVisibility` (`self.TextRender`) false false)
  (if (`KismetArrayLibrary.Array_IsValidIndex` (`self.DialogueList`) (`self.dialogIndex`))
    (bind _output_get (set `local.LastDialogue` (`|GetArrayItem` (`self.DialogueList`) (`self.dialogIndex`))))
    (`/Game/Scripts/BP/BP_Manager.DialogueOn` (`self.BP_Manager`) _output_get self (`self.NPCName`))
    (else
      (`KismetSystemLibrary.PrintString` "Add Dialogue" true true (struct :`R` 1.0 :`A` 1.0)))))

(fn `TalkEvent`
  (params (Dialogue :type "/Game/Scripts/BP/QuestSystem/Dialogue Structure"))
  (`/Game/Scripts/BP/BP_Manager.DialogueOn` (`self.BP_Manager`) Dialogue self (`self.NPCName`)))

(fn `UserConstructionScript`)